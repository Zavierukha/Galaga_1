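; Enemy Blueprint that can recolor its Ship component at random.
; The ChangeColor event creates a dynamic material instance from TEST2, randomizes its Red, Green and Blue scalar parameters, and applies it to the Ship's first material slot.
; Each call creates a new instance and stores it in DynamicMaterialRef.
; Nothing in this graph calls the event, and the construction script is empty.
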(event EventBeginPlay)

(event Collision|EventActorBeginOverlap
  (params (OtherActor :type Actor%20Object%20Reference)))

(event EventTick
  (params (DeltaSeconds :type Float%20%28single-precision%29)))

(event EventChangeColor
  (bind _returnvalue (Rendering|Material|CreateDynamicMaterialInstance "/Game/Geometry/Ships/Enemy/TEST2.TEST2" "None" "None" :!class /Script/Engine.KismetMaterialLibrary))
  (bind _output_get (Variables|Default|SetDynamic_Material_Ref _returnvalue))
  (Rendering|Material|SetScalarParameterValue _output_get "Red" (Math|Random|RandomFloatinRange 0.0 1.0) :!class /Script/Engine.MaterialInstanceDynamic)
  (Rendering|Material|SetScalarParameterValue (Variables|Default|GetDynamic_Material_Ref) "Green" (Math|Random|RandomFloatinRange 0.0 1.0) :!class /Script/Engine.MaterialInstanceDynamic)
  (Rendering|Material|SetScalarParameterValue (Variables|Default|GetDynamic_Material_Ref) "Blue" (Math|Random|RandomFloatinRange 0.0 1.0) :!class /Script/Engine.MaterialInstanceDynamic)
  (Rendering|Material|SetMaterial (Variables|Default|GetShip) 0 (Variables|Default|GetDynamic_Material_Ref)))

(fn ConstructionScript)
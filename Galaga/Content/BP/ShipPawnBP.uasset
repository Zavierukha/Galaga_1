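; Ship pawn that attaches meshes to its rocket launcher sockets at spawn and can randomize its hull color.
; BeginPlay creates the Big_Smoke and Elf mesh components at runtime, placing each at a launcher socket transform offset by its own "binding" socket, added for one and subtracted for the other.
; ChangeColor builds a dynamic material instance with random Red, Green and Blue parameters and applies it to the Ship mesh.
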(event EventBeginPlay
  (bind _ship (Variables|Default|GetShip))
  (bind _ship_2 (Variables|Default|GetShip))
  (bind _returnvalue (Transformation|GetSocketTransform _ship "Rocket_Launcher003" "RTS_Actor"))
  (bind _returnvalue_2 (Transformation|GetSocketTransform _ship_2 "Rocket_Launcher004" "RTS_Actor"))
  (bind (_location _rotation _scale) (Math|Transform|BreakTransform _returnvalue_2))
  (bind (_location_2 _rotation_2 _scale_2) (Math|Transform|BreakTransform _returnvalue))
  (Utilities|FlowControl|Sequence
    (:then_0
      (bind _returnvalue_3 (Game|AddComponentbyClass "/Script/Engine.StaticMeshComponent" false (Math|Transform|MakeTransform "0, 0, 0")))
      (Components|StaticMesh|SetStaticMesh _returnvalue_3 "/Game/Geometry/Weapons/BigSmoke/Big_Smoke.Big_Smoke")
      (Transformation|SetRelativeTransform _returnvalue_3 (Math|Transform|MakeTransform (+ _location_2 (Variables|/Script/Engine.StaticMeshSocket|GetRelativeLocation (Class|StaticMesh|FindSocket (Variables|/Script/Engine.StaticMeshComponent|GetStaticMesh _returnvalue_3) "binding"))) _rotation_2 _scale_2) false false))
    (:then_1
      (bind _returnvalue_4 (Game|AddComponentbyClass "/Script/Engine.StaticMeshComponent" false (Math|Transform|MakeTransform "0, 0, 0")))
      (Components|StaticMesh|SetStaticMesh _returnvalue_4 "/Game/Geometry/Weapons/Elf/Elf.Elf")
      (Transformation|SetRelativeTransform _returnvalue_4 (Math|Transform|MakeTransform (- _location (Variables|/Script/Engine.StaticMeshSocket|GetRelativeLocation (Class|StaticMesh|FindSocket (Variables|/Script/Engine.StaticMeshComponent|GetStaticMesh _returnvalue_4) "binding"))) _rotation _scale) false false))))

(event Collision|EventActorBeginOverlap
  (params (OtherActor :type Actor%20Object%20Reference)))

(event EventTick
  (params (DeltaSeconds :type Float%20%28single-precision%29)))

(event EventChangeColor
  (bind _returnvalue (Rendering|Material|CreateDynamicMaterialInstance "/Game/Geometry/Ships/SciFi_Fighter_AK5/TEMP.TEMP" "None" "None" :!class /Script/Engine.KismetMaterialLibrary))
  (bind _output_get (Variables|Default|SetDynamic_Material_Ref _returnvalue))
  (Rendering|Material|SetScalarParameterValue _output_get "Red" (Math|Random|RandomFloatinRange 0.0 1.0) :!class /Script/Engine.MaterialInstanceDynamic)
  (Rendering|Material|SetScalarParameterValue (Variables|Default|GetDynamic_Material_Ref) "Green" (Math|Random|RandomFloatinRange 0.0 1.0) :!class /Script/Engine.MaterialInstanceDynamic)
  (Rendering|Material|SetScalarParameterValue (Variables|Default|GetDynamic_Material_Ref) "Blue" (Math|Random|RandomFloatinRange 0.0 1.0) :!class /Script/Engine.MaterialInstanceDynamic)
  (Rendering|Material|SetMaterial (Variables|Default|GetShip) 0 (Variables|Default|GetDynamic_Material_Ref)))

(fn ConstructionScript)